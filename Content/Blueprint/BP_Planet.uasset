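; BP_Planet is a planet actor that spins on its own axis, sized and placed from Radius and CenterDistance.
; The construction script scales the mesh and offsets the actor along Y by a distance factor.
; BeginPlay moves the actor to Center and restores PlanetAxis to the original transform, making an orbit pivot.
; Tick yaws the mesh at a rate inverse to LenghtOfDay; the OrbitalPeriod-based orbit rotation is disconnected.
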(event EventBeginPlay
  (Variables|Default|SetInitial%20Planet%20Location (Transformation|GetActorTransform))
  (Transformation|SetActorLocationAndRotation (Variables|Default|GetCenter) "0, 0, 0")
  (Transformation|SetWorldLocationAndRotation (Variables|Default|GetPlanetAxis) (.location (Variables|Default|GetInitial%20Planet%20Location)) (.rotation (Variables|Default|GetInitial%20Planet%20Location)) false false))

(event Collision|EventActorBeginOverlap
  (params (OtherActor :type Actor%20Object%20Reference)))

(event EventTick
  (params (DeltaSeconds :type Float%20%28single-precision%29))
  (bind _sm_planet (Variables|Default|GetSM_Planet))
  (Transformation|SetRelativeRotation _sm_planet (Math|Rotator|MakeRotator 0.0 0.0 (+ (.yaw (Variables|/Script/Engine.SceneComponent|GetRelativeRotation _sm_planet)) (* (Utilities|Time|GetWorldDeltaSeconds) 5.0 (/ 58.0 (Variables|Default|GetLenght%20of%20Day))))) false false))

(fn ConstructionScript
  (Transformation|SetWorldScale3D (Variables|Default|GetSM_Planet) (Math|Conversions|ToVector(Float) (/ (Variables|Default|GetRadius) 1.6e+02)))
  (Transformation|SetActorLocation (Math|Vector|MakeVector 0.0 (* (Variables|Default|GetCenter%20Distance) (Variables|Default|GetDistance%20Factor)) 0.0) false false))